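; Firebolt spell ability that casts a projectile at the point under the cursor.
; On activation it waits for cursor target data, snaps the avatar to face the impact point and plays the cast montage.
; A montage gameplay event triggers SpawnProjectile toward that point, syncing the shot to the animation, with a debug print.
; The ability ends when the montage completes, is interrupted or is cancelled.
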(event `self.K2_ActivateAbility`
  (bind (_asynctaskproxy _targetdatahandle) (`TargetDataUnderCursor.CreateTargetDataUnderCursor`)
    (:`OnTargetDataReady`
      (bind _output_get (set `self.ProjectileTargetLocation` (`.ImpactPoint` (`GameplayStatics.BreakHitResult` (`AbilitySystemBlueprintLibrary.GetHitResultFromTargetData` _targetdatahandle)))))
      (`self.FaceToTarget` _output_get)
      (`AbilityTask_PlayMontageAndWait.CreatePlayMontageAndWaitProxy` "None" "/Game/Blueprints/GameplayAbilitySystem/Abilities/Fire/Firebolt/AM_Cast_Firebolt.AM_Cast_Firebolt"
        (:`then`
          (`AbilityTask_WaitGameplayEvent.WaitGameplayEvent` (struct :`TagName` "Event.Montage.Firebolt") null
            (:`EventReceived`
              (`self.SpawnProjectile` (`self.ProjectileTargetLocation`))
              (`KismetSystemLibrary.PrintString` "Spawn"))))
        (:`OnCompleted`
          (`self.K2_EndAbility` :!label _label))
        (:`OnInterrupted`
          (goto _label))
        (:`OnCancelled`
          (goto _label))))))

(fn `FaceToTarget`
  (params (TargetLocation :type "Vector Structure"))
  (bind _returnvalue (`self.GetAvatarActorFromActorInfo`))
  (`Actor.K2_SetActorRotation` _returnvalue (`KismetMathLibrary.MakeRotFromX` (- TargetLocation (`Actor.K2_GetActorLocation` _returnvalue))) false))